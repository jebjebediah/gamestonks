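; BP_Dollar is a money pickup that scatters when spawned and disappears if not collected within seven seconds.
; On BeginPlay it starts the despawn timer and eases its root to a random nearby XY point at a fixed height with random yaw, then enables overlap events on its Box.
; When a ThirdPersonCharacter overlaps it, it passes its Amount to PickupMoney and destroys itself.
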(event Custom|Destroy%20Money
  (Actor|DestroyActor))

(event Collision|EventActorBeginOverlap
  (params (OtherActor :type Actor%20Object%20Reference))
  (bind _asthird_person_character (Utilities|Casting|CastToThirdPersonCharacter OtherActor))
  (Default|PickupMoney _asthird_person_character (Variables|Default|GetAmount))
  (Actor|DestroyActor))

(event EventBeginPlay
  (bind _returnvalue (Transformation|GetActorRotation))
  (bind _returnvalue_2 (Transformation|GetActorLocation))
  (Utilities|Time|SetTimerbyEvent (delegate Custom|Destroy%20Money) 7.0)
  (Components|MoveComponentTo (Variables|Default|GetDefaultSceneRoot) (Math|Vector|MakeVector (+ (.x _returnvalue_2) (Math|Random|RandomFloatinRange -3e+02 3e+02)) (+ (.y _returnvalue_2) (Math|Random|RandomFloatinRange -3e+02 3e+02)) 2.1e+02) (Math|Rotator|MakeRotator (.roll _returnvalue) (.pitch _returnvalue) (Math|Random|RandomFloatinRange -3.6e+02 3.6e+02)) true false 1.0 false)
  (Variables|/Script/Engine.PrimitiveComponent|SetbGenerateOverlapEvents (Variables|Default|GetBox) true))

(fn ConstructionScript)